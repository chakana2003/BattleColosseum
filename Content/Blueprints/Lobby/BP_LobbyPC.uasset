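; Lobby player controller that manages each player's profile, lobby menu and chat in a multiplayer lobby.
; CreateMyInfo loads name and icon from the save, sets host or preparing status by authority, creates WB_Lobby and calls CallUpdate.
; BP_LobbyGM handles character spawning, king selection and the player list for chat fan-out, while receive events refresh the widget.
; It also toggles the menu, labels the pawn, saves profile data and has hardcoded X/Z message keys.
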(event `CreateMyInfo`
  (bind _myinfo (`self.MyInfo`))
  ;[1 1 1] Create MyInfo
  (`/Engine/EditorBlueprintResources/StandardMacros.IsValid` (`self.SaveGameRef`)
    (:`Is Valid`
      _)
    (:`Is Not Valid`
      (bind _returnvalue (`GameplayStatics.CreateSaveGameObject` "/Script/BattleColosseum.C_SaveGame"))
      (set `self.SaveGameRef` _returnvalue)))
  (bind _returnvalue_2 (`GameplayStatics.LoadGameFromSlot` (`C_SaveGame.SaveGameName` (`self.SaveGameRef`))))
  (bind _asc_save_game (cast `C_SaveGame` _returnvalue_2))
  (bind _output_get (set `self.SaveGameRef` _asc_save_game))
  (if (`self.HasAuthority`)
    (bind (_myinfo_name _myinfo_icon) (break `C_S_PlayerInfo` (`C_SaveGame.MyInfo` _output_get)))
    (bind _structout (setmembers `C_S_PlayerInfo` :`StructRef` _myinfo :`Name` _myinfo_name :`Icon` _myinfo_icon :`status` "방장" :`SelectCharacter` (make `C_S_Characters` "/Game/PlayerIcon/Sumnail/SUM_No.SUM_No" "/Game/Blueprints/BP_NullCharacter.BP_NullCharacter_C" "/Game/Blueprints/BP_NullCharacter.BP_NullCharacter_C")))
    (set `self.MyInfo` _structout)
    (else
      (bind _structout_2 (setmembers `C_S_PlayerInfo` :`StructRef` _myinfo :`Name` _myinfo_name :`Icon` _myinfo_icon :`status` "준비중..." :`SelectCharacter` (make `C_S_Characters` "/Game/PlayerIcon/Sumnail/SUM_No.SUM_No" "/Game/Blueprints/BP_NullCharacter.BP_NullCharacter_C" "/Game/Blueprints/BP_NullCharacter.BP_NullCharacter_C")))
      (set `self.MyInfo` _structout_2)))
  (`self.SetupLobbyMenu`)
  (`self.CallUpdate` (`self.MyInfo`)))

(event `CallUpdate`
  (params (NewInfo :type "C_S_PlayerInfo Structure"))
  ;[1 1 1] Call Update
  (bind _output_get (set `self.MyInfo` NewInfo))
  (bind _asbp_lobby_gm (cast `/Game/Blueprints/Lobby/BP_LobbyGM` (`GameplayStatics.GetGameMode`)))
  (`/Game/Blueprints/Lobby/BP_LobbyGM.SpawnCharacter` _asbp_lobby_gm self (`.LobbyCharacter` (break `C_S_Characters` (`.SelectCharacter` (break `C_S_PlayerInfo` _output_get)))))
  (`/Game/Blueprints/Lobby/BP_LobbyGM.EveryoneUpdate` _asbp_lobby_gm))

(event `Key|X`
  (params (Key :type "Key Structure"))
  (:`Pressed`
    (`/Game/UI/Lobby/WB_Lobby.GoMassage` (`self.LobbyWidget`) "오호홍")))

(event `Key|Z`
  (params (Key :type "Key Structure"))
  (:`Pressed`
    (`/Game/UI/Lobby/WB_Lobby.GoMassage` (`self.LobbyWidget`) "성호병신")))

(event `InputAction|K_OpenLobbyMenu`
  (params (Key :type "Key Structure"))
  (bind _lobbywidget (`self.LobbyWidget`))
  (:`Pressed`
    (`/Engine/EditorBlueprintResources/StandardMacros.FlipFlop`
      (:`A`
        (`UserWidget.PlayAnimation` _lobbywidget (`/Game/UI/Lobby/WB_Lobby.InMenu` _lobbywidget) 0.0 1 "Forward" 1.0)
        (set `self.bShowMouseCursor` true)
        (`WidgetBlueprintLibrary.SetInputMode_GameAndUIEx` self _lobbywidget))
      (:`B`
        (`UserWidget.PlayAnimation` _lobbywidget (`/Game/UI/Lobby/WB_Lobby.OutMenu` _lobbywidget) 0.0 1 "Forward" 1.0)
        (set `self.bShowMouseCursor` false)
        (`WidgetBlueprintLibrary.SetInputMode_GameOnly` self)))))

(event `UpdatePlayerCount`
  (params (NewCount :type Integer))
  ;[1 1 1] Update Player Count
  (set `/Game/UI/Lobby/WB_Lobby.PlayerCount` (`KismetTextLibrary.Conv_IntToText` NewCount) (`self.LobbyWidget`)))

(event `SetConnectedPlayerInfo`
  (params (`New PlayerInfos` :type "Array of C_S_PlayerInfo Structure"))
  ;[1 1 1] SetConnectedPlayerInfo
  (set `self.ConnectedPlayerInfo` `New PlayerInfos`)
  (`/Game/UI/Lobby/WB_Lobby.ClearPlayerList` (`self.LobbyWidget`))
  (for _array_element (`self.ConnectedPlayerInfo`)
    (`/Game/UI/Lobby/WB_Lobby.CreatePlayerWindow` (`self.LobbyWidget`) _array_element)))

(event `ShowLoadingScreen`
  ;[1 1 1] ShowLoadingScreen
  (`Widget.RemoveFromParent` (`self.LobbyWidget`))
  (`WidgetBlueprintLibrary.SetInputMode_GameOnly` self))

(event `KingSelectedRecieve`
  (params (NewKingStatus :type Boolean))
  ;[1 1 1] KingSelectedRecieve
  (`Widget.SetIsEnabled` (`/Game/UI/Lobby/WB_Lobby.King` (`self.LobbyWidget`)) NewKingStatus))

(event `SettingUserID`
  (bind _returnvalue (`self.K2_GetPawn`))
  (bind _myinfo_name (break `C_S_PlayerInfo` (`self.MyInfo`)))
  (bind _asbp_null_character (cast `/Game/Blueprints/BP_NullCharacter` _returnvalue)
    (:`then`
      (`TextRenderComponent.K2_SetText` (`C_NullCharacter.UserID` _asbp_null_character) _myinfo_name))
    (:`CastFailed`
      (bind _asc_lobby_character (cast `C_LobbyCharacter` _returnvalue))
      (`TextRenderComponent.K2_SetText` (`C_LobbyCharacter.UserID` _asc_lobby_character) _myinfo_name))))

(event `KingSelectSend`
  (params (NewState :type Boolean))
  ;[1 1 1] KingSelectSend
  (`/Game/Blueprints/Lobby/BP_LobbyGM.SetKing` (cast `/Game/Blueprints/Lobby/BP_LobbyGM` (`GameplayStatics.GetGameMode`) :!pure true) NewState))

(event `SendChatMassage`
  (params (SendingText :type Text))
  (bind _myinfo_name (break `C_S_PlayerInfo` (`self.MyInfo`)))
  ;[1 1 1] SendChatMassage
  (set `self.SendText` SendingText)
  (set `self.SenderText` _myinfo_name)
  (bind _asbp_lobby_gm (cast `/Game/Blueprints/Lobby/BP_LobbyGM` (`GameplayStatics.GetGameMode`)))
  (for _array_element (`/Game/Blueprints/Lobby/BP_LobbyGM.ConnectedPlayer` _asbp_lobby_gm)
    (`self.UpdateChatWindow` _array_element (`self.SenderText`) (`self.SendText`))))

(event `UpdateChatWindow`
  (params (Sender :type Text) (Text :type Text))
  ;[1 1 1] UpdateChatWindow
  (`/Game/UI/Lobby/WB_ChatWindow.UpdateChatScroll` (`/Game/UI/Lobby/WB_Lobby.WB_ChatWindow` (`self.LobbyWidget`)) Sender Text))

(fn `SaveGame`
  (bind _savegameref (`self.SaveGameRef`))
  (`/Engine/EditorBlueprintResources/StandardMacros.IsValid` (`self.SaveGameRef`)
    (:`Is Valid`
      _)
    (:`Is Not Valid`
      (bind _returnvalue (`GameplayStatics.CreateSaveGameObject` "/Script/BattleColosseum.C_SaveGame"))
      (set `self.SaveGameRef` _returnvalue)))
  (set `C_SaveGame.MyInfo` (`self.MyInfo`) _savegameref)
  (`GameplayStatics.SaveGameToSlot` _savegameref (`C_SaveGame.SaveGameName` _savegameref)))

(fn `SaveSelectedCharacter`
  (params (SelectedCharacter :type "C_S_Characters Structure"))
  (bind _savegameref (`self.SaveGameRef`))
  (`/Engine/EditorBlueprintResources/StandardMacros.IsValid` (`self.SaveGameRef`)
    (:`Is Valid`
      _)
    (:`Is Not Valid`
      (bind _returnvalue (`GameplayStatics.CreateSaveGameObject` "/Script/BattleColosseum.C_SaveGame"))
      (set `self.SaveGameRef` _returnvalue)))
  (setmembers `C_S_PlayerInfo` :`StructRef` (`C_SaveGame.MyInfo` _savegameref) :`SelectCharacter` SelectedCharacter)
  (`GameplayStatics.SaveGameToSlot` _savegameref (`C_SaveGame.SaveGameName` _savegameref)))

(fn `SetupLobbyMenu`
  (`/Engine/EditorBlueprintResources/StandardMacros.IsValid` (`self.LobbyWidget`)
    (:`Is Valid`
      _)
    (:`Is Not Valid`
      (bind _returnvalue (`|CreateWidget` "/Game/UI/Lobby/WB_Lobby.WB_Lobby_C"))
      (set `self.LobbyWidget` _returnvalue)))
  (`UserWidget.AddToViewport` (`self.LobbyWidget`) 0))

(fn `UserConstructionScript`)