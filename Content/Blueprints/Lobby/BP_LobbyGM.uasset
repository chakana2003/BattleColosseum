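; Lobby game mode that tracks connected players, spawns their chosen characters and decides whether the match can start.
; On login it registers each lobby controller; character spawning replaces the current pawn with one at a random spot and yaw inside the BP_SpawnBox.
; EveryoneUpdate gathers player info and pushes it, the player count and King availability to every controller.
; It then sets CanStart only if everyone, host included, has picked a character.
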(event `SetKing`
  (params (KingStatus :type Boolean))
  ;[1 1 1] SetKing
  (set `self.AvaliableKing` KingStatus))

(event `self.K2_PostLogin`
  (params (NewPlayer :type "PlayerController Object Reference"))
  ;[1 1 1] 플레이어 입장 시
  (`/Engine/EditorBlueprintResources/StandardMacros.IsValid` (`self.SpawnPoint`)
    (:`Is Valid`
      _)
    (:`Is Not Valid`
      (bind _outactors (`GameplayStatics.GetAllActorsOfClass` "/Game/Blueprints/Lobby/BP_SpawnBox.BP_SpawnBox_C"))
      (set `self.SpawnPoint` (`|GetArrayItem` _outactors))))
  (bind _asbp_lobby_pc (cast `/Game/Blueprints/Lobby/BP_LobbyPC` NewPlayer))
  (`KismetArrayLibrary.Array_Add` (`self.ConnectedPlayer`) _asbp_lobby_pc)
  (`/Game/Blueprints/Lobby/BP_LobbyPC.CreateMyInfo` _asbp_lobby_pc))

(event `SpawnCharacter`
  (params (PlayerController :type "/Game/Blueprints/Lobby/BP_LobbyPC Object Reference") (Character :type "Pawn Class Reference"))
  (bind _returnvalue (`Controller.K2_GetPawn` PlayerController))
  (bind _spawnpoint (`self.SpawnPoint`))
  ;[1 1 1] SpawnCharacter
  (`/Engine/EditorBlueprintResources/StandardMacros.IsValid` _returnvalue ; 컨트롤하고있는 Pawn이 존재하는지
    (:`Is Valid`
      (`self.K2_DestroyActor` _returnvalue) ; 존재하면 없애버리고
    )
    (:`Is Not Valid`
      _))
  (bind _returnvalue_2 (`|SpawnActorFromClass` Character (`KismetMathLibrary.MakeTransform` (`KismetMathLibrary.RandomPointInBoundingBox` (`self.K2_GetActorLocation` _spawnpoint) (`BoxComponent.BoxExtent` (`/Game/Blueprints/Lobby/BP_SpawnBox.Box` _spawnpoint))) (`KismetMathLibrary.MakeRotator` 0.0 0.0 (`KismetMathLibrary.RandomFloatInRange` 0.0 360.0))) "Undefined" "OverrideRootScale" null null))
  (`Controller.Possess` PlayerController _returnvalue_2))

(event `EveryoneUpdate`
  (bind _connectedplayer (`self.ConnectedPlayer`))
  ;[1 1 1] Everyone Update
  (set `self.PlayerCount` (`KismetArrayLibrary.Array_Length` (`self.ConnectedPlayer`)))
  (`KismetArrayLibrary.Array_Clear` (`self.ConnectedPlayerInfo`))
  (for _array_element _connectedplayer
    (`KismetArrayLibrary.Array_Add` (`self.ConnectedPlayerInfo`) (`/Game/Blueprints/Lobby/BP_LobbyPC.MyInfo` _array_element))
    (`/Game/Blueprints/Lobby/BP_LobbyPC.UpdatePlayerCount` _array_element (`self.PlayerCount`)))
  (for _array_element_2 _connectedplayer
    (`/Game/Blueprints/Lobby/BP_LobbyPC.SetConnectedPlayerInfo` _array_element_2 (`self.ConnectedPlayerInfo`)) ; 업데이트된 플레이어들의 정보를 클라이언트에게 전달
    (`/Game/Blueprints/Lobby/BP_LobbyPC.KingSelectedRecieve` _array_element_2 (`self.AvaliableKing`)) ; 킹 사용 가능 여부 클라이언트에게 전달
  )
  (set `self.CanStart` true)
  (for _array_element_3 (`self.ConnectedPlayerInfo`)
    (if (== (`.GameCharacter` (break `C_S_Characters` (`.SelectCharacter` (break `C_S_PlayerInfo` _array_element_3)))) "/Game/Blueprints/BP_NullCharacter.BP_NullCharacter_C")
      (set `self.CanStart` false :!label _label)))
  (if (`self.CanStart`)
    (bind _asbp_lobby_pc (cast `/Game/Blueprints/Lobby/BP_LobbyPC` (`GameplayStatics.GetPlayerController` 0)))
    (if (== (`.GameCharacter` (break `C_S_Characters` (`.SelectCharacter` (break `C_S_PlayerInfo` (`/Game/Blueprints/Lobby/BP_LobbyPC.MyInfo` _asbp_lobby_pc))))) "/Game/Blueprints/BP_NullCharacter.BP_NullCharacter_C")
      (goto _label)
      (else
        (set `self.CanStart` true)))))

(fn `OnRep_ConnectedPlayer`)

(fn `UserConstructionScript`)