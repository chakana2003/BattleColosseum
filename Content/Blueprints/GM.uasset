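; GM is a Game Mode that tracks logged-in PC controllers, feeds player data to the HUD and runs a match countdown.
; PostLogin creates each widget and starts a 0.01s timer gathering all pawns, names and locations, sent after the loop via the last controller.
; BeginPlay timers call IIIIII on every controller once, then push and decrement GameState LeftTime each second.
; An unconnected chain would respawn players as their selected characters.
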(event `self.K2_PostLogin`
  (params (NewPlayer :type "PlayerController Object Reference"))
  (bind _aspc (cast `/Game/Blueprints/PC` NewPlayer))
  (`/Game/Blueprints/PC.CreateWidget` _aspc)
  (`KismetArrayLibrary.Array_Add` (`self.ConnectedPlayer`) _aspc)
  (`KismetSystemLibrary.Delay` 1.0)
  (`KismetSystemLibrary.K2_SetTimerDelegate` (delegate `Do`) 0.01 true))

(event `self.ReceiveTick`
  (params (DeltaSeconds :type "Float (single-precision)")))

(event `Do`
  (`KismetArrayLibrary.Array_Clear` (`self.Names`))
  (`KismetArrayLibrary.Array_Clear` (`self.Pawns`))
  (`KismetArrayLibrary.Array_Clear` (`self.Locations`))
  (for _array_element (`self.ConnectedPlayer`)
    (bind _returnvalue (`Controller.K2_GetPawn` _array_element))
    (`KismetArrayLibrary.Array_Add` (`self.Pawns`) _returnvalue)
    (bind _myinfo_0_name (break `C_S_PlayerInfo` (`/Game/Blueprints/PC.MyInfo_0` _array_element)))
    (`KismetArrayLibrary.Array_Add` (`self.Names`) _myinfo_0_name)
    (`KismetArrayLibrary.Array_Add` (`self.Locations`) (`self.K2_GetActorLocation` _returnvalue)))
  (`/Game/Blueprints/PC.SendToHUD` _array_element (`self.Pawns`) (`self.Names`) (`self.Locations`)))

(event `self.ReceiveBeginPlay`
  (`KismetSystemLibrary.K2_SetTimerDelegate` (delegate `Inie`) 1.0)
  (`KismetSystemLibrary.K2_SetTimerDelegate` (delegate `Popie`) 1.0 true))

(event `Inie`
  (bind _asgm (cast `/Game/Blueprints/GM` (`GameplayStatics.GetGameMode`)))
  (for _array_element (`/Game/Blueprints/GM.ConnectedPlayer` _asgm)
    (`/Game/Blueprints/PC.IIIIII` _array_element)))

(event `Popie`
  (bind _asgs (cast `/Game/Blueprints/GS` (`GameplayStatics.GetGameState`) :!pure true))
  (bind _lefttime (`/Game/Blueprints/GS.LeftTime` _asgs))
  (bind _asgm (cast `/Game/Blueprints/GM` (`GameplayStatics.GetGameMode`)))
  (for _array_element (`/Game/Blueprints/GM.ConnectedPlayer` _asgm)
    (`/Game/Blueprints/PC.PPPPPP` _array_element "승주야왜안돼" (`KismetTextLibrary.Conv_DoubleToText` _lefttime "HalfToEven")))
  (set `/Game/Blueprints/GS.LeftTime` (- _lefttime 1.0) _asgs))

(fn `UserConstructionScript`)