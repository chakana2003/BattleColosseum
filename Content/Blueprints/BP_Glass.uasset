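; BP_Glass is a breakable glass actor with a Glass component and a Box collider.
; BreakGlass checks that Glass is still valid, sets the Box to ignore all channels, spawns a muzzle-flash particle with random rotation and scale at the glass, then destroys the Glass component.
; The event graph is empty, including AnyDamage, so nothing in this Blueprint calls BreakGlass itself.
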(event `self.ReceiveAnyDamage`
  (params (Damage :type "Float (single-precision)") (DamageType :type "DamageType Object Reference") (InstigatedBy :type "Controller Object Reference") (DamageCauser :type "Actor Object Reference")))

(fn `BreakGlass`
  (bind _returnvalue (`KismetMathLibrary.RandomFloatInRange` 0.3 0.5))
  (bind _returnvalue_2 (`KismetMathLibrary.RandomFloatInRange` 0.0 360.0))
  (`/Engine/EditorBlueprintResources/StandardMacros.IsValid` (`self.Glass`)
    (:`Is Valid`
      (`PrimitiveComponent.SetCollisionResponseToAllChannels` (`self.Box`) "ECR_Ignore")
      (`GameplayStatics.SpawnEmitterAtLocation` "/Game/InfinityBladeEffects/Effects/FX_Monsters/FX_Monster_Gruntling/Master/P_BackPack_MuzzleFlash.P_BackPack_MuzzleFlash" (`SceneComponent.K2_GetComponentLocation` (`self.Glass`)) (`KismetMathLibrary.MakeRotator` _returnvalue_2 _returnvalue_2 _returnvalue_2) (`KismetMathLibrary.MakeVector` _returnvalue _returnvalue _returnvalue))
      (`ActorComponent.K2_DestroyComponent` (`self.Glass`)))))

(fn `UserConstructionScript`)