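; Game instance Blueprint that handles front-end menu flow and level travel.
; SaveGameCheck looks for a save slot and shows the main menu if one exists, otherwise the create-player screen.
; Both show functions create and cache their widget on first use, add it to the viewport and enable the mouse cursor.
; Instance_MoveToLevel changes maps by running a servertravel console command with the given destination.
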(event `Instance_MoveToLevel`
  (params (Destation :type String))
  (`KismetSystemLibrary.ExecuteConsoleCommand` (`KismetStringLibrary.Concat_StrStr` "servertravel " Destation) (`GameplayStatics.GetPlayerController` 0)))

(fn `SaveGameCheck`
  (bind _returnvalue (`GameplayStatics.DoesSaveGameExist` (`self.SAVEGAME`)))
  (if _returnvalue
    (`self.ShowMainMenu`)
    (else
      (`self.ShowCreatePlayer`))))

(fn `ShowCreatePlayer`
  (bind _returnvalue (`GameplayStatics.GetPlayerController` 0))
  (`/Engine/EditorBlueprintResources/StandardMacros.IsValid` (`self.CreatePlayer`)
    (:`Is Valid`
      _)
    (:`Is Not Valid`
      (bind _returnvalue_2 (`|CreateWidget` "/Game/UI/MainMenu/WB_CreatePlayer.WB_CreatePlayer_C" _returnvalue))
      (set `self.CreatePlayer` _returnvalue_2)))
  (`UserWidget.AddToViewport` (`self.CreatePlayer`) 0)
  (set `PlayerController.bShowMouseCursor` true _returnvalue))

(fn `ShowMainMenu`
  (bind _returnvalue (`GameplayStatics.GetPlayerController` 0))
  (`/Engine/EditorBlueprintResources/StandardMacros.IsValid` (`self.MainMenu`)
    (:`Is Valid`
      _)
    (:`Is Not Valid`
      (bind _returnvalue_2 (`|CreateWidget` "/Game/UI/MainMenu/WB_MainMenuM.WB_MainMenuM_C" _returnvalue))
      (set `self.MainMenu` _returnvalue_2)))
  (`UserWidget.AddToViewport` (`self.MainMenu`) 0)
  (set `PlayerController.bShowMouseCursor` true _returnvalue))