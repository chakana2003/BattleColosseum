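; BP_NullCharacter is a character Blueprint that drives its static mesh's material from movement speed and prints a debug message on BeginPlay.
; Tick periodically samples per-frame displacement, then lerps between the previous and new samples at a rate set by DeltaSec.
; The clamped result feeds the "Max" and "Min" scalar parameters, with Min trailing Max.
; Logic to set UserID text from the lobby controller's player name is disconnected.
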(event `self.ReceiveBeginPlay`
  (`KismetSystemLibrary.PrintString` "NULL 나왓땅~!" true true (struct :`R` 0.463542 :`G` 0.407313 :`A` 1.0) 10.0))

(event `self.ReceiveTick`
  (params (DeltaSeconds :type "Float (single-precision)"))
  (bind _lerpaph (`self.LerpAph`))
  (bind _returnvalue (* (`self.TotalSpeedLength`) 0.5))
  (if (>= (`self.LerpAph`) 1.0)
    (set `self.LerpAph` 0.0)
    (bind _output_get (set `self.NewPos` (`self.K2_GetActorLocation`)))
    (set `self.OldVelo` (`self.NewVelo`))
    (set `self.NewVelo` (`KismetMathLibrary.VSize` (- (`self.OldPos`) _output_get)))
    (else
      (set `self.LerpAph` (+ _lerpaph (* DeltaSeconds (`self.deltaSec`))))
      (set `self.TotalSpeedLength` (`KismetMathLibrary.Lerp` (`self.OldVelo`) (`self.NewVelo`) _lerpaph))
      (`MeshComponent.SetScalarParameterValueOnMaterials` (`self.StaticMesh`) "Max" (`KismetMathLibrary.FClamp` _returnvalue 0.1 100.0))
      (`MeshComponent.SetScalarParameterValueOnMaterials` (`self.StaticMesh`) "Min" (`KismetMathLibrary.FClamp` (- _returnvalue 5.0) 0.1 100.0))
      (set `self.OldPos` (`self.K2_GetActorLocation`)))))

(fn `UserConstructionScript`)