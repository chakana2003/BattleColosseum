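; BP_PlayGM is the play game mode Blueprint, relaying countdown and setup events to BP_WonseokPC player controllers.
; Timer events loop over connected controllers to show, update and hide a countdown, reading BP_PlayGS for remaining time and choosing a game-start or character-creation label.
; Per-player events create the play widget or send begin-play to the controller and its warrior pawn.
; CreateSpawnBox caches the TriggerBox tagged FirstSpawn.
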(event `self.SendCurrentPC`
  (params (Player :type "PlayerController Object Reference"))
  (`KismetSystemLibrary.PrintString` "Send Current PC Call" true true (struct :`G` 0.66 :`B` 1.0 :`A` 1.0) 10.0)
  (bind _asbp_wonseok_pc (cast `/Game/Blueprints/Play/BP_WonseokPC` Player))
  (`/Game/Blueprints/Play/BP_WonseokPC.CreatePlayWidget` _asbp_wonseok_pc))

(event `self.BeginStartTimer`
  ;[1 1 1] 카운트다운
  (for _array_element (`self.ConnectedPlayerControllers`)
    (bind _asbp_wonseok_pc (cast `/Game/Blueprints/Play/BP_WonseokPC` _array_element))
    (`/Game/Blueprints/Play/BP_WonseokPC.InCount` _asbp_wonseok_pc)))

(event `self.PopStartTimer`
  (bind _asbp_play_gs (cast `/Game/Blueprints/Play/BP_PlayGS` (`GameplayStatics.GetGameState`) :!pure true))
  (bind _returnvalue (`KismetTextLibrary.Conv_DoubleToText` (`C_PlayGS.LeftStartTime` _asbp_play_gs) "HalfToEven"))
  ;[1 1 1] 카운트다운
  (for _array_element (`self.ConnectedPlayerControllers`)
    (bind _asbp_wonseok_pc (cast `/Game/Blueprints/Play/BP_WonseokPC` _array_element))
    (if (`C_PlayGS.PreStart` _asbp_play_gs)
      (`/Game/Blueprints/Play/BP_WonseokPC.DoCount` _asbp_wonseok_pc "게임 시작까지..." _returnvalue)
      (else
        (`/Game/Blueprints/Play/BP_WonseokPC.DoCount` _asbp_wonseok_pc "캐릭터 생성까지..." _returnvalue)))))

(event `self.EndStartTimer`
  ;[1 1 1] 카운트다운
  (for _array_element (`self.ConnectedPlayerControllers`)
    (bind _asbp_wonseok_pc (cast `/Game/Blueprints/Play/BP_WonseokPC` _array_element))
    (`/Game/Blueprints/Play/BP_WonseokPC.OutCount` _asbp_wonseok_pc)))

(event `self.SendWarriorFromCode`
  (params (Player :type "PlayerController Object Reference"))
  (bind _asbp_wonseok_pc (cast `/Game/Blueprints/Play/BP_WonseokPC` Player))
  (`/Game/Wonseok/NewInventory/Test_PC.SendBeginPlayToCilent` _asbp_wonseok_pc)
  (bind _asmy_c_warrior_wonseok (cast `/Game/Wonseok/MyC_Warrior_Wonseok` (`Controller.K2_GetPawn` Player)))
  (`/Game/Wonseok/MyC_Warrior_Wonseok.SendBeginPlayToPawn` _asmy_c_warrior_wonseok))

(fn `CreateSpawnBox`
  (`/Engine/EditorBlueprintResources/StandardMacros.IsValid` (`self.SpaningBox`)
    (:`Is Valid`
      _)
    (:`Is Not Valid`
      (bind _outactors (`GameplayStatics.GetAllActorsWithTag` "FirstSpawn"))
      (set `self.SpaningBox` (cast `TriggerBox` (`|GetArrayItem` _outactors) :!pure true))))
  (return))

(fn `UserConstructionScript`)