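; BP_PlayPC is the play-mode player controller that holds the player's info, including name and selected character.
; PassCharacterServer stores the incoming info and has BP_PlayGM spawn the lobby character for this controller, passing along the old controller.
; A Load function, not called here, restores that info from the SAVEGAME slot.
; Key C prints the name and character classes; Z, on authority, calls the game mode's Spawn.
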(event `self.ReceiveBeginPlay`)

(event `PassCharacterServer`
  (params (OldPC :type "PlayerController Object Reference") (NewInfo :type "C_S_PlayerInfo Structure"))
  ;[1 0.6936 0.6537] PassCharacterServer
  (set `self.MyInfo` NewInfo)
  (bind _asbp_play_gm (cast `/Game/Blueprints/Play/BP_PlayGM` (`GameplayStatics.GetGameMode`)))
  (`/Game/Blueprints/Play/BP_PlayGM.SpawnCharacter(Ver Wait)` _asbp_play_gm OldPC self (`.LobbyCharacter` (break `C_S_Characters` (`.SelectCharacter` (break `C_S_PlayerInfo` (`self.MyInfo`)))))))

(event `Key|C`
  (params (Key :type "Key Structure"))
  (bind _myinfo (`self.MyInfo`))
  (:`Pressed`
    (`KismetSystemLibrary.PrintString` (`KismetStringLibrary.Concat_StrStr` "Name : " (`KismetTextLibrary.Conv_TextToString` (break `C_S_PlayerInfo` _myinfo)) "/LCharacter : " (`KismetSystemLibrary.GetClassDisplayName` (`.LobbyCharacter` (break `C_S_Characters` (`.SelectCharacter` (break `C_S_PlayerInfo` _myinfo))))) " /GCharacter : " (`KismetSystemLibrary.GetClassDisplayName` (`.GameCharacter` (break `C_S_Characters` (`.SelectCharacter` (break `C_S_PlayerInfo` _myinfo)))))) true true (struct :`G` 0.66 :`B` 1.0 :`A` 1.0) 10.0)))

(event `Key|Z`
  (params (Key :type "Key Structure"))
  (:`Pressed`
    (`/Engine/EditorBlueprintResources/ActorMacros.Switch Has Authority`
      (:`Authority`
        (bind _asbp_play_gm (cast `/Game/Blueprints/Play/BP_PlayGM` (`GameplayStatics.GetGameMode`)))
        (`/Game/Blueprints/Play/BP_PlayGM.Spawn` _asbp_play_gm)))))

(fn `Load`
  (bind _returnvalue (`GameplayStatics.LoadGameFromSlot` "SAVEGAME"))
  (bind _asc_save_game (cast `C_SaveGame` _returnvalue))
  (set `self.MyInfo` (`C_SaveGame.MyInfo` _asc_save_game))
  (`KismetSystemLibrary.PrintString` "Load Success!!" true true (struct :`R` 1.0 :`G` 0.054508 :`A` 1.0) 30.0))

(fn `UserConstructionScript`)