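; BP_WonseokWarrior is a warrior Blueprint that drives camera shake and spawns a temporary trigger capsule.
; Pressing 8 spawns a TriggerCapsule_Blueprint with a ten-second lifespan.
; While Came is true, the shake event starts a looping timer that repeatedly shakes the first player's camera, periodically re-randomizing the intensity.
; The timer clears itself once it finds Came false.
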(event `self.ReceiveBeginPlay`
  (`parent.ReceiveBeginPlay`)
  (set `self.scale` (`KismetMathLibrary.RandomFloatInRange` 0.0 2.0)))

(event `Key|Eight`
  (params (Key :type "Key Structure"))
  (:`Pressed`
    (bind _returnvalue (`|SpawnActorFromClass` "/Game/sinyoung/TriggerCapsule_Blueprint.TriggerCapsule_Blueprint_C" (`KismetMathLibrary.MakeTransform` (0.0 0.0 0.0)) "Undefined" "OverrideRootScale" null null))
    (`self.SetLifeSpan` _returnvalue 10.0)))

(event `shake`
  (if (`self.came`)
    (bind _returnvalue (`KismetSystemLibrary.K2_SetTimerDelegate` (delegate `Custom Event_0`) 0.5 true))
    (set `self.timer handle` _returnvalue)))

(event `Custom Event_0`
  (if (`self.came`)
    (set `self.time` (+ (`self.time`) 0.5))
    (if (>= (`self.time`) 2.0)
      (set `self.time` 0.0)
      (set `self.scale` (`KismetMathLibrary.RandomFloatInRange` 0.0 2.0)))
    (`PlayerController.ClientStartCameraShake` :`self` (`GameplayStatics.GetPlayerController` 0) :`Shake` "/Game/Wonseok/warrior_sinyoung/widget/camerashake.camerashake_C" :`Scale` (`self.scale`))
    (else
      (`KismetSystemLibrary.K2_ClearAndInvalidateTimerHandle` (`self.timer handle`)))))

(fn `UserConstructionScript`
  (`parent.UserConstructionScript`))