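; BP_WonseokPC is a player controller for the play session that owns the WB_PlayM HUD widget and includes debug keys.
; Events create the widget and forward countdown show, update and hide calls to it.
; BroadBurningAreaClient shows a fire-arrow alert for a numbered zone.
; Debug keys print player info and, with authority only, dump the game mode's burning areas or toggle a cursor-enabled dev panel.
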(event `Key|V`
  (params (Key :type "Key Structure"))
  ;[1 1 1] 디버그
  (:`Pressed`
    (`/Engine/EditorBlueprintResources/ActorMacros.Switch Has Authority`
      (:`Authority`
        (bind _asbp_play_gm (cast `/Game/Blueprints/Play/BP_PlayGM` (`GameplayStatics.GetGameMode`)))
        (for _array_element (`C_PlayGM.BurningAreas` _asbp_play_gm)
          (`KismetSystemLibrary.PrintString` (`KismetStringLibrary.Concat_StrStr` "Area : " (`KismetStringLibrary.Conv_NameToString` (`|GetArrayItem` (`Actor.Tags` _array_element) 1)) " Damage : " (`KismetStringLibrary.Conv_DoubleToString` (`PainCausingVolume.DamagePerSec` _array_element))) true true (struct :`R` 1.0 :`B` 0.099114 :`A` 1.0) 10.0))))))

(event `Key|C`
  (params (Key :type "Key Structure"))
  (bind _myinfo (`self.MyInfo`))
  ;[1 1 1] 디버그
  (:`Pressed`
    (`KismetSystemLibrary.PrintString` (`KismetStringLibrary.Concat_StrStr` (`KismetTextLibrary.Conv_TextToString` (break `C_S_PlayerInfo` _myinfo)) "/" (`KismetSystemLibrary.GetClassDisplayName` (`.LobbyCharacter` (break `C_S_Characters` (`.SelectCharacter` (break `C_S_PlayerInfo` _myinfo))))) "/" (`KismetSystemLibrary.GetClassDisplayName` (`.GameCharacter` (break `C_S_Characters` (`.SelectCharacter` (break `C_S_PlayerInfo` _myinfo))))) "/" (`KismetSystemLibrary.GetDisplayName` (`self.K2_GetPawn`)) "/" (`KismetSystemLibrary.GetDisplayName` self)))))

(event `CreatePlayWidget`
  (`/Engine/EditorBlueprintResources/StandardMacros.IsValid` (`self.PlayWidgetRef`)
    (:`Is Valid`
      _)
    (:`Is Not Valid`
      (bind _returnvalue (`|CreateWidget` "/Game/UI/Play/WB_PlayM.WB_PlayM_C" self))
      (set `self.PlayWidgetRef` _returnvalue)))
  (`UserWidget.AddToViewport` (`self.PlayWidgetRef`) 0)
  (`KismetSystemLibrary.PrintString` "Create Widget!" true true (struct :`G` 0.66 :`B` 1.0 :`A` 1.0) 10.0))

(event `InCount`
  (`/Game/UI/Play/WB_PlayM.InCountDownBox` (`self.PlayWidgetRef`)))

(event `Key|P`
  (params (Key :type "Key Structure"))
  (bind _playwidgetref (`self.PlayWidgetRef`))
  ;[1 1 1] 디버그
  (:`Pressed`
    (`/Engine/EditorBlueprintResources/ActorMacros.Switch Has Authority`
      (:`Authority`
        (`/Engine/EditorBlueprintResources/StandardMacros.FlipFlop`
          (:`A`
            (set `self.bShowMouseCursor` true)
            (`WidgetBlueprintLibrary.SetInputMode_GameAndUIEx` self)
            (`UserWidget.PlayAnimation` _playwidgetref (`/Game/UI/Play/WB_PlayM.InDev` _playwidgetref) 0.0 1 "Forward" 1.0))
          (:`B`
            (set `self.bShowMouseCursor` false)
            (`WidgetBlueprintLibrary.SetInputMode_GameOnly` self)
            (`UserWidget.PlayAnimation` _playwidgetref (`/Game/UI/Play/WB_PlayM.OutDev` _playwidgetref) 0.0 1 "Forward" 1.0)))))))

(event `DoCount`
  (params (Text :type Text) (Numb :type Text))
  (`/Game/UI/Play/WB_PlayM.DoCountDown` (`self.PlayWidgetRef`) Text Numb))

(event `OutCount`
  (`/Game/UI/Play/WB_PlayM.OutCountDownBox` (`self.PlayWidgetRef`)))

(event `BroadBurningAreaClient`
  (params (Order :type Name))
  (`/Game/UI/Play/WB_PlayM.SideBroadMassage` (`self.PlayWidgetRef`) (`KismetTextLibrary.Conv_StringToText` (`KismetStringLibrary.Concat_StrStr` (`KismetStringLibrary.Conv_NameToString` Order) "번 구역에")) "불화살이 쏟아집니다!" true))

(fn `UserConstructionScript`
  (`parent.UserConstructionScript`))