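; MyHUD is a HUD that draws floating name tags over pawns.
; The SendPawn event stores arrays of pawns, names and locations, though drawing uses locations only to check that data exists.
; Each DrawHUD projects live pawn positions, skips those behind the camera, and draws centered, raised, translucent text.
; Text scales inversely with distance from the player's pawn, so nearer names appear larger.
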(event `/Game/Blueprints/BPI.SendPawn`
  (params (Pawns :type "Array of Pawn Object Reference (by ref)") (Names :type "Array of Text (by ref)") (Locations :type "Array of Vector Structure (by ref)"))
  (set `self.AllPawns` Pawns)
  (set `self.AllNames` Names)
  (set `self.AllLocations` Locations))

(event `self.ReceiveDrawHUD`
  (params (SizeX :type Integer) (SizeY :type Integer))
  (set `self.ScreenSize` (`KismetMathLibrary.MakeVector2D` (`KismetMathLibrary.Conv_IntToDouble` SizeX) (`KismetMathLibrary.Conv_IntToDouble` SizeY)))
  (if (`KismetArrayLibrary.Array_IsValidIndex` (`self.AllLocations`))
    (for (_array_element _array_index) (`self.AllPawns`)
      (bind _returnvalue (`self.K2_GetActorLocation` _array_element))
      (bind (_returnvalue_x _returnvalue_y _returnvalue_z) (`KismetMathLibrary.BreakVector` (`self.Project` _returnvalue)))
      (if (> _returnvalue_z 0.0)
        (bind _returnvalue_2 (`KismetTextLibrary.Conv_TextToString` (`|GetArrayItem` (`self.AllNames`) _array_index)))
        (bind _returnvalue_3 (/ 2000.0 (`KismetMathLibrary.VSize` (- (`self.K2_GetActorLocation` (`GameplayStatics.GetPlayerPawn` 0)) _returnvalue))))
        (bind (_outwidth _outheight) (`self.GetTextSize` _returnvalue_2 "/Game/Fonts/BMYEONSUNG_ttf_Font.BMYEONSUNG_ttf_Font" _returnvalue_3))
        (`self.DrawText` _returnvalue_2 (struct :`R` 1.0 :`G` 1.0 :`B` 1.0 :`A` 0.8) (- _returnvalue_x (/ _outwidth 2.0)) (- _returnvalue_y (* _outheight 3.0)) "/Game/Fonts/BMYEONSUNG_ttf_Font.BMYEONSUNG_ttf_Font" _returnvalue_3)))))

(fn `UserConstructionScript`)