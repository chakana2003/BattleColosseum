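; Door actor that swings open when something overlaps its Trigger component and swings shut when the overlap ends.
; DoorOpen and DoorClose set the IsOpen flag and reset Speed, which serves as the interpolation alpha.
; Tick lerps the Door's relative yaw between closed and a quarter turn, advancing by a fixed per-frame step.
; Motion is frame-rate dependent, and reversing mid-swing jumps to the opposite endpoint.
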(event `self.ReceiveTick`
  (params (DeltaSeconds :type "Float (single-precision)"))
  (if (>= (`self.Speed`) 1.0)
    _
    (elif (`self.isOpen`)
      (`SceneComponent.K2_SetRelativeRotation` (`self.Door`) (`KismetMathLibrary.MakeRotator` 0.0 0.0 (`KismetMathLibrary.Lerp` 0.0 90.0 (`self.Speed`))) false false)
      (set `self.Speed` (+ (`self.Speed`) 0.01))
      (else
        (`SceneComponent.K2_SetRelativeRotation` (`self.Door`) (`KismetMathLibrary.MakeRotator` 0.0 0.0 (`KismetMathLibrary.Lerp` 90.0 0.0 (`self.Speed`))) false false)
        (set `self.Speed` (+ (`self.Speed`) 0.01))))))

(event `self.Trigger.OnComponentBeginOverlap`
  (params (OverlappedComponent :type "PrimitiveComponent Object Reference") (OtherActor :type "Actor Object Reference") (OtherComp :type "PrimitiveComponent Object Reference") (OtherBodyIndex :type Integer) (bFromSweep :type Boolean) (SweepResult :type "HitResult Structure (by ref)"))
  (`self.DoorOpen`))

(event `self.Trigger.OnComponentEndOverlap`
  (params (OverlappedComponent :type "PrimitiveComponent Object Reference") (OtherActor :type "Actor Object Reference") (OtherComp :type "PrimitiveComponent Object Reference") (OtherBodyIndex :type Integer))
  (`self.DoorClose`))

(fn `DoorClose`
  (set `self.isOpen` false)
  (set `self.Speed` 0.0))

(fn `DoorOpen`
  (set `self.isOpen` true)
  (set `self.Speed` 0.0))

(fn `UserConstructionScript`)