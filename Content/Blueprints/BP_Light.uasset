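; BP_Light is a light actor whose point light constantly jitters in position, paired with a particle system.
; Tick picks a random relative X/Z target in a small box, then lerps the light toward it from its current location.
; The Speed variable serves as the lerp alpha, growing with delta time and triggering a new target once past one.
; TurnSwitch toggles visibility of both light and particles.
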(event `self.ReceiveBeginPlay`
  (set `self.Speed` 2.0))

(event `self.ReceiveTick`
  (params (DeltaSeconds :type "Float (single-precision)"))
  (bind _returnvalue_location (`KismetMathLibrary.BreakTransform` (`SceneComponent.GetRelativeTransform` (`self.PointLight`))))
  (if (> (`self.Speed`) 1.0)
    (set `self.NewLoc` (`KismetMathLibrary.MakeVector` (`KismetMathLibrary.RandomFloatInRange` 450.0 550.0) 0.0 (`KismetMathLibrary.RandomFloatInRange` 750.0 850.0)))
    (set `self.Speed` 0.0)
    (else
      (`SceneComponent.K2_SetRelativeLocation` (`self.PointLight`) (`KismetMathLibrary.VLerp` _returnvalue_location (`self.NewLoc`) (`self.Speed`)) false false)
      (set `self.Speed` (+ (`self.Speed`) (* 10.0 (`GameplayStatics.GetWorldDeltaSeconds`)))))))

(fn `TurnSwitch`
  (`SceneComponent.ToggleVisibility` (`self.PointLight`) false)
  (`SceneComponent.ToggleVisibility` (`self.ParticleSystem`) false))

(fn `UserConstructionScript`)