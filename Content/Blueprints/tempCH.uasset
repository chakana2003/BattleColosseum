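; tempCH is a player-controlled pawn Blueprint that appears to be a test of basic movement and camera look input.
; The K_MoveForward axis adds movement along fixed world +Y, regardless of facing, and K_LookUp feeds controller pitch.
; Tick prints any non-zero K_LookUp value for debugging.
; Disconnected nodes hold alternatives for spring arm pitch and controller roll or yaw, which never run.
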(event `InputAxis|K_MoveForward`
  (params (AxisValue :type "Float (single-precision)"))
  (`self.AddMovementInput` (0.0 1.0 0.0) AxisValue))

(event `self.ReceiveTick`
  (params (DeltaSeconds :type "Float (single-precision)"))
  (bind _returnvalue (`self.GetInputAxisValue`))
  (if (!= _returnvalue 0.0)
    (`KismetSystemLibrary.PrintString` (`KismetStringLibrary.Conv_DoubleToString` _returnvalue))))

(event `InputAxis|K_LookUp`
  (params (AxisValue :type "Float (single-precision)"))
  (`|ExecutionSequence`
    (:`then_2`
      (`self.AddControllerPitchInput` AxisValue))))

(fn `UserConstructionScript`)