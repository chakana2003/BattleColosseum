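; BP_Enemy is an AI enemy pawn with health and a peace, chase, attack or dead state.
; Seeing a pawn through PawnSensing while at peace stores it and starts the chase, while damage that empties health triggers death.
; SetState writes the state to the Blackboard and sets walk speed per state.
; It also refills health on every transition and ignores changes once dead.
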(event `self.ReceiveBeginPlay`
  (set `self.CurrentHp` (`self.MaxHp`))
  (`self.Set State` "NewEnumerator0"))

(event `self.ReceiveAnyDamage`
  (params (Damage :type "Float (single-precision)") (DamageType :type "DamageType Object Reference") (InstigatedBy :type "Controller Object Reference") (DamageCauser :type "Actor Object Reference"))
  (bind _output_get (set `self.CurrentHp` (- (`self.CurrentHp`) Damage)))
  (if (> _output_get 0.0)
    (`KismetSystemLibrary.PrintString` (`KismetStringLibrary.Conv_DoubleToString` (`self.CurrentHp`)))
    (else
      (`self.Set State` "NewEnumerator3"))))

(event `self.PawnSensing.OnSeePawn`
  (params (Pawn :type "Pawn Object Reference"))
  (if (`|EnumEquality` (`self.CurrentStatePawn `) "NewEnumerator0")
    (set `self.Instigator` Pawn)
    (`self.Set State` "NewEnumerator1")))

(fn `Set State`
  (params (NewParam :type "/Game/Sinyoung/pratice/BPE_EnemyState Enum" :default "NewEnumerator0"))
  (bind _charactermovement (`self.CharacterMovement`))
  (if (`|EnumInequality` (`self.CurrentStatePawn `) "NewEnumerator3")
    (bind _output_get (set `self.CurrentStatePawn ` NewParam))
    (set `self.CurrentHp` (`self.MaxHp`))
    (`|ExecutionSequence`
      (:`then_0`
        (`BlackboardComponent.SetValueAsEnum` (`AIBlueprintHelperLibrary.GetBlackboard` (`self.GetController`)) (`self.StateKey`) _output_get))
      (:`then_1`
        (switch `/Game/Sinyoung/pratice/BPE_EnemyState` _output_get
          (:`NewEnumerator0`
            (set `CharacterMovementComponent.MaxWalkSpeed` 300.0 _charactermovement))
          (:`NewEnumerator1`
            (set `CharacterMovementComponent.MaxWalkSpeed` 600.0 _charactermovement))
          (:`NewEnumerator2`
            (set `CharacterMovementComponent.MaxWalkSpeed` 0.0 _charactermovement))
          (:`NewEnumerator3`
            (set `CharacterMovementComponent.MaxWalkSpeed` 0.0 _charactermovement)))))))

(fn `UserConstructionScript`)