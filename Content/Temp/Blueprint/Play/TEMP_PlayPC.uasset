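; Player controller for play that restores the player's saved character choice and gets that character spawned.
; On BeginPlay, the local controller clears all widgets and loads PlayerInfo from the TEMPSAVE slot through TEMP_SaveGame.
; It passes that info to PassCharacterIntoServer, which stores it and asks TEMP_PlayGM to spawn the chosen character for this controller.
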(event `self.ReceiveBeginPlay`
  (if (`self.IsLocalController`)
    (`WidgetLayoutLibrary.RemoveAllWidgets`)
    (`self.Load`)
    (`self.PassCharacterIntoServer` (`self.PlayerInfo`))))

(event `PassCharacterIntoServer`
  (params (CharacterInfo :type "/Game/Temp/Blueprint/TEMP_PlayerInfo Structure"))
  ;[1 1 1] passCharacterIntoServer
  (set `self.PlayerInfo` CharacterInfo)
  (bind _astemp_play_gm (cast `/Game/Temp/Blueprint/Play/TEMP_PlayGM` (`GameplayStatics.GetGameMode`)))
  (`/Game/Temp/Blueprint/Play/TEMP_PlayGM.SpawnCharacter` _astemp_play_gm self (break `/Game/Temp/Blueprint/TEMP_Character` (`.ChoiceCharacter_12_195468EB474C43A353D23CB66709BA61` (break `/Game/Temp/Blueprint/TEMP_PlayerInfo` (`self.PlayerInfo`))))))

(fn `Load`
  (bind _returnvalue (`GameplayStatics.LoadGameFromSlot` (`self.TEMPSAVE`)))
  (bind _astemp_save_game (cast `/Game/Temp/Blueprint/TEMP_SaveGame` _returnvalue))
  (set `self.PlayerInfo` (`/Game/Temp/Blueprint/TEMP_SaveGame.PlayerInfo` _astemp_save_game)))

(fn `UserConstructionScript`)