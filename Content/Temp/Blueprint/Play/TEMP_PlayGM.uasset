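; Temporary play GameMode that spawns player pawns and handles logout in a session-based game.
; It caches all PlayerStarts on BeginPlay and records controllers passed through OnSwapPlayerControllers in a list.
; SpawnCharacter destroys the controller's current pawn, spawns the given class at a random PlayerStart with random yaw, then possesses it.
; On logout of a TEMP_PlayPC, it calls DestroySession for that controller.
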(event `self.ReceiveBeginPlay`
  (bind _outactors (`GameplayStatics.GetAllActorsOfClass` "/Script/Engine.PlayerStart"))
  (set `self.SpawnPoint` _outactors))

(event `self.K2_OnSwapPlayerControllers`
  (params (OldPC :type "PlayerController Object Reference") (NewPC :type "PlayerController Object Reference"))
  ;[1 1 1] OnSwapPlayerControllers
  (`KismetArrayLibrary.Array_Add` (`self.AllPlayerControllers`) NewPC))

(event `SpawnCharacter`
  (params (Controller :type "PlayerController Object Reference") (Character :type "Character Class Reference"))
  (bind _returnvalue (`Controller.K2_GetPawn` Controller))
  (bind _spawnpoint (`self.SpawnPoint`))
  ;[1 1 1] SpawnCharacter
  (`/Engine/EditorBlueprintResources/StandardMacros.IsValid` _returnvalue
    (:`Is Valid`
      (`self.K2_DestroyActor` _returnvalue))
    (:`Is Not Valid`
      _))
  (bind _returnvalue_2 (`|SpawnActorFromClass` Character (`KismetMathLibrary.MakeTransform` (`self.K2_GetActorLocation` (`|GetArrayItem` _spawnpoint (`KismetMathLibrary.RandomIntegerInRange` 0 (- (`KismetArrayLibrary.Array_Length` _spawnpoint) 1)))) (`KismetMathLibrary.MakeRotator` 0.0 0.0 (`KismetMathLibrary.RandomFloatInRange` 0.0 360.0))) "Undefined" "OverrideRootScale" null null))
  (`Controller.Possess` Controller _returnvalue_2))

(event `self.K2_OnLogout`
  (params (ExitingController :type "Controller Object Reference"))
  ;[1 1 1] OnLogout
  (bind _astemp_play_pc (cast `/Game/Temp/Blueprint/Play/TEMP_PlayPC` ExitingController))
  (`DestroySessionCallbackProxy.DestroySession` (cast `/Game/Temp/Blueprint/TEMP_BCGI` (`GameplayStatics.GetGameInstance`) :!pure true) _astemp_play_pc))

(fn `UserConstructionScript`)