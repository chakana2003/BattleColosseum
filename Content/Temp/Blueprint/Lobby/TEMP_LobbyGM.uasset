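; Lobby game mode that tracks connected TEMP_LobbyPC players and gates the start of the match.
; EveryoneUpdate pushes player count, player infos and king availability to every controller, then sets CanStart from character choices, overwriting it per player so only the last player and player 0 decide.
; SpawnCharacter replaces a player's pawn at a random PlayerStart with random yaw.
; LaunchGame calls MoveWorld to load Map_Main.
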(event `self.K2_PostLogin`
  (params (NewPlayer :type "PlayerController Object Reference"))
  (bind _astemp_lobby_pc (cast `/Game/Temp/Blueprint/Lobby/TEMP_LobbyPC` NewPlayer))
  (`KismetArrayLibrary.Array_Add` (`self.ConnectedPlayer`) _astemp_lobby_pc)
  (`/Game/Temp/Blueprint/Lobby/TEMP_LobbyPC.CreateMyInfo` _astemp_lobby_pc))

(event `SetKing`
  (params (King :type Boolean))
  (set `self.AvaliableKing` King))

(event `self.K2_OnLogout`
  (params (ExitingController :type "Controller Object Reference"))
  (bind _astemp_lobby_pc (cast `/Game/Temp/Blueprint/Lobby/TEMP_LobbyPC` ExitingController))
  (`KismetArrayLibrary.Array_RemoveItem` (`self.ConnectedPlayer`) _astemp_lobby_pc)
  (`self.EveryoneUpdate`))

(event `EveryoneUpdate`
  (bind _connectedplayer (`self.ConnectedPlayer`))
  ;[1 1 1] EveryoneUpdate
  (set `self.CurrentPlayer` (`KismetArrayLibrary.Array_Length` (`self.ConnectedPlayer`)))
  (`KismetArrayLibrary.Array_Clear` (`self.ConnectedPlayerInfo`))
  (for _array_element _connectedplayer
    (`KismetArrayLibrary.Array_Add` (`self.ConnectedPlayerInfo`) (`/Game/Temp/Blueprint/Lobby/TEMP_LobbyPC.MyInfo` _array_element))
    (`/Game/Temp/Blueprint/Lobby/TEMP_LobbyPC.UpdatePlayerCount` _array_element (`self.CurrentPlayer`)))
  (for _array_element_2 _connectedplayer
    (`/Game/Temp/Blueprint/Lobby/TEMP_LobbyPC.SetConnectedPlayerInfo` _array_element_2 (`self.ConnectedPlayerInfo`))
    (`/Game/Temp/Blueprint/Lobby/TEMP_LobbyPC.KingSelectRecieve` _array_element_2 (`self.AvaliableKing`)))
  (for _array_element_3 (`self.ConnectedPlayerInfo`)
    (if (== (break `/Game/Temp/Blueprint/TEMP_Character` (`.ChoiceCharacter_12_195468EB474C43A353D23CB66709BA61` (break `/Game/Temp/Blueprint/TEMP_PlayerInfo` _array_element_3))) "/Game/Blueprints/BP_NullCharacter.BP_NullCharacter_C")
      (set `self.CanStart` false :!label _label)
      (else
        (bind _astemp_lobby_pc (cast `/Game/Temp/Blueprint/Lobby/TEMP_LobbyPC` (`GameplayStatics.GetPlayerController` 0)))
        (if (== (break `/Game/Temp/Blueprint/TEMP_Character` (`.ChoiceCharacter_12_195468EB474C43A353D23CB66709BA61` (break `/Game/Temp/Blueprint/TEMP_PlayerInfo` (`/Game/Temp/Blueprint/Lobby/TEMP_LobbyPC.MyInfo` _astemp_lobby_pc)))) "/Game/Blueprints/BP_NullCharacter.BP_NullCharacter_C")
          (goto _label)
          (else
            (set `self.CanStart` true)))))))

(event `SpawnCharacter`
  (params (PlayerController :type "PlayerController Object Reference") (Character :type "Character Class Reference"))
  (bind _returnvalue (`Controller.K2_GetPawn` PlayerController))
  (bind _startpoint (`self.StartPoint`))
  ;[1 1 1] SpawnCharacter
  (`/Engine/EditorBlueprintResources/StandardMacros.IsValid` _returnvalue
    (:`Is Valid`
      (`self.K2_DestroyActor` _returnvalue))
    (:`Is Not Valid`
      _))
  (bind _returnvalue_2 (`|SpawnActorFromClass` Character (`KismetMathLibrary.MakeTransform` (`self.K2_GetActorLocation` (`|GetArrayItem` _startpoint (`KismetMathLibrary.RandomIntegerInRange` 0 (- (`KismetArrayLibrary.Array_Length` _startpoint) 1)))) (`KismetMathLibrary.MakeRotator` 0.0 0.0 (`KismetMathLibrary.RandomFloatInRange` 0.0 360.0))) "Undefined" "OverrideRootScale" null null))
  (`Controller.Possess` PlayerController _returnvalue_2))

(event `LaunchGame`
  ;[1 1 1] LaunchGame
  (`self.MoveWorld` "Map_Main")
  (`KismetSystemLibrary.PrintString` "Hello"))

(event `self.ReceiveBeginPlay`
  (bind _outactors (`GameplayStatics.GetAllActorsOfClass` "/Script/Engine.PlayerStart")) ; StartPoint 를 저장
  (set `self.StartPoint` _outactors))

(fn `UserConstructionScript`)