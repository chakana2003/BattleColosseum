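; Lobby player controller that manages each player's menu, info, chat and character selection in a multiplayer lobby.
; CreateMyInfo loads name and icon from the save slot, builds the lobby widget, then CallUpdate has TEMP_LobbyGM spawn the character and refresh everyone.
; Player list, count, King button and chat updates drive the widget, while chat sends loop over the GameMode's connected controllers.
; It also toggles menu input, saves character choice and shows a loading screen.
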(event `InputAction|K_OpenLobby`
  (params (Key :type "Key Structure"))
  (bind _lobbymenuref (`self.LobbyMenuRef`))
  (:`Pressed`
    (`/Engine/EditorBlueprintResources/StandardMacros.FlipFlop`
      (:`A`
        (`UserWidget.PlayAnimation` _lobbymenuref (`/Game/Temp/UI/TEMP_LobbyMenu.InMenu` _lobbymenuref) 0.0 1 "Forward" 1.0)
        (set `self.bShowMouseCursor` true)
        (`WidgetBlueprintLibrary.SetInputMode_GameAndUIEx` self _lobbymenuref))
      (:`B`
        (`UserWidget.PlayAnimation` _lobbymenuref (`/Game/Temp/UI/TEMP_LobbyMenu.OutMenu` _lobbymenuref) 0.0 1 "Forward" 1.0)
        (set `self.bShowMouseCursor` false)
        (`WidgetBlueprintLibrary.SetInputMode_GameOnly` self)))))

(event `self.ReceiveBeginPlay`)

(event `CreateMyInfo`
  ;[1 1 1] CreateMyInfo
  (bind _returnvalue (`GameplayStatics.LoadGameFromSlot` (`self.TEMPSAVE`)))
  (bind _astemp_save_game (cast `/Game/Temp/Blueprint/TEMP_SaveGame` _returnvalue))
  (bind (_playerinfo_name _playerinfo_icon) (break `/Game/Temp/Blueprint/TEMP_PlayerInfo` (`/Game/Temp/Blueprint/TEMP_SaveGame.PlayerInfo` _astemp_save_game)))
  (bind _structout (setmembers `/Game/Temp/Blueprint/TEMP_PlayerInfo` :`StructRef` (`self.MyInfo`) :`Name` _playerinfo_name :`Icon` _playerinfo_icon :`ChoiceCharacter` (make `/Game/Temp/Blueprint/TEMP_Character` "/Game/Blueprints/BP_NullCharacter.BP_NullCharacter_C" "/Game/InfinityBladeEffects/Effects/FX_Textures/Texture/Basic_WhiteBar01.Basic_WhiteBar01")))
  (`self.SetupLobbyMenu`)
  (`self.CallUpdate` _structout))

(event `CallUpdate`
  (params (PlayerInfo :type "/Game/Temp/Blueprint/TEMP_PlayerInfo Structure"))
  ;[1 1 1] CallUpdate
  (bind _output_get (set `self.MyInfo` PlayerInfo))
  (bind _astemp_lobby_gm (cast `/Game/Temp/Blueprint/Lobby/TEMP_LobbyGM` (`GameplayStatics.GetGameMode`)))
  (`/Game/Temp/Blueprint/Lobby/TEMP_LobbyGM.SpawnCharacter` _astemp_lobby_gm self (break `/Game/Temp/Blueprint/TEMP_Character` (`.ChoiceCharacter_12_195468EB474C43A353D23CB66709BA61` (break `/Game/Temp/Blueprint/TEMP_PlayerInfo` _output_get))))
  (`/Game/Temp/Blueprint/Lobby/TEMP_LobbyGM.EveryoneUpdate` _astemp_lobby_gm))

(event `KingSelectRecieve`
  (params (Status :type Boolean))
  (`Widget.SetIsEnabled` (`/Game/Temp/UI/TEMP_LobbyMenu.King` (`self.LobbyMenuRef`)) Status))

(event `KingSelectSend`
  (params (KingBool :type Boolean))
  (`/Game/Temp/Blueprint/Lobby/TEMP_LobbyGM.SetKing` (cast `/Game/Temp/Blueprint/Lobby/TEMP_LobbyGM` (`GameplayStatics.GetGameMode`) :!pure true) KingBool))

(event `UpdatePlayerCount`
  (params (PlayerCount :type Integer))
  ;[1 1 1] UpdatePlayerCount
  (set `/Game/Temp/UI/TEMP_LobbyMenu.PlayerCount` (`KismetTextLibrary.Conv_IntToText` PlayerCount) (`self.LobbyMenuRef`)))

(event `SetConnectedPlayerInfo`
  (params (ConnectedPlayers :type "Array of /Game/Temp/Blueprint/TEMP_PlayerInfo Structure"))
  ;[1 1 1] SetConnectedPlayerInfo
  (set `self.ConnectedPlayerInfo` ConnectedPlayers)
  (`/Game/Temp/UI/TEMP_LobbyMenu.ClearPlayerList` (`self.LobbyMenuRef`))
  (for _array_element (`self.ConnectedPlayerInfo`)
    (`/Game/Temp/UI/TEMP_LobbyMenu.CreatePlayerWindow` (`self.LobbyMenuRef`) _array_element)))

(event `SendChatMassage`
  (params (SendingMessage :type Text))
  (bind _myinfo_name (break `/Game/Temp/Blueprint/TEMP_PlayerInfo` (`self.MyInfo`)))
  ;[1 1 1] SendChatMassage
  (set `self.TextSend` SendingMessage)
  (set `self.TextSender` _myinfo_name)
  (bind _astemp_lobby_gm (cast `/Game/Temp/Blueprint/Lobby/TEMP_LobbyGM` (`GameplayStatics.GetGameMode`)))
  (for _array_element (`/Game/Temp/Blueprint/Lobby/TEMP_LobbyGM.ConnectedPlayer` _astemp_lobby_gm)
    (`self.UpdateChatWindow` _array_element (`self.TextSender`) (`self.TextSend`))))

(event `UpdateChatWindow`
  (params (Sender :type Text) (Text :type Text))
  ;[1 1 1] UpdateChatWindow
  (`/Game/Temp/UI/TEMP_ChatWindow.UpdateChatScroll` (`/Game/Temp/UI/TEMP_LobbyMenu.TEMP_ChatWindow` (`self.LobbyMenuRef`)) Sender Text))

(event `ShowLoadingScreen`
  ;[1 1 1] ShowLoadingScreen
  (`Widget.RemoveFromParent` (`self.LobbyMenuRef`))
  (bind _returnvalue (`|CreateWidget` "/Game/Temp/UI/TEMP_Loading.TEMP_Loading_C" self))
  (`UserWidget.AddToViewport` _returnvalue 0))

(fn `SaveSelectedCharacter`
  (params (SelectedCharacter :type "Character Class Reference") (Sumnail :type "Texture2D Object Reference"))
  (bind _returnvalue (`GameplayStatics.CreateSaveGameObject` "/Game/Temp/Blueprint/TEMP_SaveGame.TEMP_SaveGame_C"))
  (bind _output_get (set `self.SaveGameRef` _returnvalue))
  (setmembers `/Game/Temp/Blueprint/TEMP_PlayerInfo` :`StructRef` (`/Game/Temp/Blueprint/TEMP_SaveGame.PlayerInfo` _output_get) :`ChoiceCharacter` (make `/Game/Temp/Blueprint/TEMP_Character` SelectedCharacter Sumnail))
  (`GameplayStatics.SaveGameToSlot` (`self.SaveGameRef`) (`self.TEMPSAVE`)))

(fn `SetupLobbyMenu`
  (`/Engine/EditorBlueprintResources/StandardMacros.IsValid` (`self.LobbyMenuRef`)
    (:`Is Valid`
      _)
    (:`Is Not Valid`
      (bind _returnvalue (`|CreateWidget` "/Game/Temp/UI/TEMP_LobbyMenu.TEMP_LobbyMenu_C"))
      (set `self.LobbyMenuRef` _returnvalue)))
  (`UserWidget.AddToViewport` (`self.LobbyMenuRef`) 0))

(fn `UserConstructionScript`)