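; TEMP_BCGI is a temporary Blueprint that picks the menu to show based on whether a saved game exists.
; SaveGameCheck looks for the TEMPSAVE slot and calls ShowMainMenu if found, otherwise ShowCreateMenu for player creation.
; Both show functions lazily create and cache their widget for the first player controller, add it to the viewport and enable the mouse cursor.
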(fn `SaveGameCheck`
  (bind _returnvalue (`GameplayStatics.DoesSaveGameExist` (`self.TEMPSAVE`)))
  (if _returnvalue
    (`self.ShowMainMenu`)
    (else
      (`self.ShowCreateMenu`))))

(fn `ShowCreateMenu`
  (bind _returnvalue (`GameplayStatics.GetPlayerController` 0))
  (`/Engine/EditorBlueprintResources/StandardMacros.IsValid` (`self.CreatePlayerW`)
    (:`Is Valid`
      _)
    (:`Is Not Valid`
      (bind _returnvalue_2 (`|CreateWidget` "/Game/Temp/UI/TEMP_CreatePlayer.TEMP_CreatePlayer_C" _returnvalue))
      (set `self.CreatePlayerW` _returnvalue_2)))
  (`UserWidget.AddToViewport` (`self.CreatePlayerW`) 0)
  (set `PlayerController.bShowMouseCursor` true _returnvalue))

(fn `ShowMainMenu`
  (bind _returnvalue (`GameplayStatics.GetPlayerController` 0))
  (`/Engine/EditorBlueprintResources/StandardMacros.IsValid` (`self.MainMenuW`)
    (:`Is Valid`
      _)
    (:`Is Not Valid`
      (bind _returnvalue_2 (`|CreateWidget` "/Game/Temp/UI/TEMP_MainMenu.TEMP_MainMenu_C" _returnvalue))
      (set `self.MainMenuW` _returnvalue_2)))
  (`UserWidget.AddToViewport` (`self.MainMenuW`) 0)
  (set `PlayerController.bShowMouseCursor` true _returnvalue))