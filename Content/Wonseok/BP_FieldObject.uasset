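; BP_FieldObject is a field object that can be farmed for item drops, with its mesh async-loaded from FieldObjectTable by ItemClassID.
; Warrior overlap with Sphere1 tracks the player and toggles an outline made from a duplicate mesh component with a dynamic material.
; EndPharmingCreateItem handles two IDs, spawning a physics-simulated Master_Item, then animating material Amount by timeline before destroying the actor.
; Name widget creation is disconnected, though Tick still positions it.
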(event `Itemname`)

(event `self.ReceiveBeginPlay`
  (if (!= (`self.ItemClassID`) 0)
    (bind _returnvalue (`|GetDataTableRow` "/Game/Wonseok/FieldObjectTable.FieldObjectTable" (`KismetStringLibrary.Conv_StringToName` (`KismetStringLibrary.Conv_IntToString` (`self.ItemClassID`))))
      (:`then`
        (bind _object (`|LoadAsset` (`.StaticMesh_15_39E7277D40AF6AA92A42139964542626` (break `/Game/Wonseok/FieldObjectClass` _returnvalue)))
          (:`Completed`
            (bind _asstatic_mesh (cast `StaticMesh` _object))
            (bind _output_get (set `self.Mesh` _asstatic_mesh))
            (`StaticMeshComponent.SetStaticMesh` (`self.StaticMesh`) _output_get)))))))

(event `CreateOutline`
  (if (not (`self.HasOutline?`))
    (bind _returnvalue (`AddComponent|NODE_AddStaticMeshComponent-0` :`bManualAttachment` true :`RelativeTransform` (`SceneComponent.K2_GetComponentToWorld` (`self.StaticMesh`))))
    (bind _output_get (set `self.MeshComponent` _returnvalue))
    (`StaticMeshComponent.SetStaticMesh` _output_get (`self.Mesh`))
    (bind _returnvalue_2 (`PrimitiveComponent.CreateDynamicMaterialInstance` _output_get 0 "/Game/Wonseok/M_Outline_Inst.M_Outline_Inst"))
    (`MaterialInstanceDynamic.SetVectorParameterValue` _returnvalue_2 "Color" (`self.Color`))
    (`MaterialInstanceDynamic.SetScalarParameterValue` _returnvalue_2 "Scale" (`self.Scale`))
    (set `self.HasOutline?` true)))

(event `self.ReceiveTick`
  (params (DeltaSeconds :type "Float (single-precision)"))
  (bind _itemnamewidget (`self.ItemNameWidget`))
  (bind (_screenlocation _returnvalue) (`PlayerController.ProjectWorldLocationToScreen` (`GameplayStatics.GetPlayerController` 0) (`self.K2_GetActorLocation`) false))
  (`/Engine/EditorBlueprintResources/StandardMacros.IsValid` _itemnamewidget
    (:`Is Valid`
      (if _returnvalue
        (`UserWidget.SetPositionInViewport` _itemnamewidget _screenlocation true)))))

(event `self.Sphere1.OnComponentBeginOverlap`
  (params (OverlappedComponent :type "PrimitiveComponent Object Reference") (OtherActor :type "Actor Object Reference") (OtherComp :type "PrimitiveComponent Object Reference") (OtherBodyIndex :type Integer) (bFromSweep :type Boolean) (SweepResult :type "HitResult Structure (by ref)"))
  (bind _asmy_c_warrior_wonseok (cast `/Game/Wonseok/MyC_Warrior_Wonseok` OtherActor))
  (set `self.InPlayer1` _asmy_c_warrior_wonseok)
  (`KismetArrayLibrary.Array_Add` (`self.InPlayers`) _asmy_c_warrior_wonseok)
  (`self.CreateOutline`))

(event `DeleteOutline`
  (bind _meshcomponent (`self.MeshComponent`))
  (`/Engine/EditorBlueprintResources/StandardMacros.IsValid` _meshcomponent
    (:`Is Valid`
      (`ActorComponent.K2_DestroyComponent` _meshcomponent)
      (set `self.HasOutline?` false))))

(event `addtoview`)

(event `self.Sphere1.OnComponentEndOverlap`
  (params (OverlappedComponent :type "PrimitiveComponent Object Reference") (OtherActor :type "Actor Object Reference") (OtherComp :type "PrimitiveComponent Object Reference") (OtherBodyIndex :type Integer))
  (bind _asmy_c_warrior_wonseok (cast `/Game/Wonseok/MyC_Warrior_Wonseok` OtherActor))
  (`KismetArrayLibrary.Array_RemoveItem` (`self.InPlayers`) _asmy_c_warrior_wonseok)
  (`self.DeleteOutline`))

(event `removewidget`)

(event `EndPharmingCreateItem`
  (bind _staticmesh (`self.StaticMesh`))
  (`self.DeleteOutline`)
  (if (== (`self.ItemClassID`) 101)
    (bind _returnvalue (`|SpawnActorFromClass` "/Game/Wonseok/Master_Item.Master_Item_C" (`self.GetTransform`) "Undefined" "OverrideRootScale" null 3 0.0 0.0 false null))
    (`PrimitiveComponent.SetSimulatePhysics` (`/Game/Wonseok/Master_Item.StaticMesh` _returnvalue) true)
    (bind _returnvalue_2 (`PrimitiveComponent.CreateDynamicMaterialInstance` _staticmesh 0 null))
    (bind _returnvalue_3 (`PrimitiveComponent.CreateDynamicMaterialInstance` _staticmesh 1 null))
    (bind (_direction `_새_트랙_0`) (`Timeline|타임라인_0`)
      (:`Update`
        (`MaterialInstanceDynamic.SetScalarParameterValue` _returnvalue_2 "Amount" `_새_트랙_0`)
        (`MaterialInstanceDynamic.SetScalarParameterValue` _returnvalue_3 "Amount" `_새_트랙_0`))
      (:`Finished`
        (`self.K2_DestroyActor`)))
    (elif (== (`self.ItemClassID`) 103)
      (bind _returnvalue_4 (`|SpawnActorFromClass` "/Game/Wonseok/Master_Item.Master_Item_C" (`self.GetTransform`) "Undefined" "OverrideRootScale" null 4 0.0 0.0 false null))
      (`PrimitiveComponent.SetSimulatePhysics` (`/Game/Wonseok/Master_Item.StaticMesh` _returnvalue_4) true)
      (bind _returnvalue_5 (`PrimitiveComponent.CreateDynamicMaterialInstance` (`self.StaticMesh`) 0 null))
      (bind (_direction_2 `_새_트랙_0_2`) (`Timeline|타임라인_1`)
        (:`Update`
          (`MaterialInstanceDynamic.SetScalarParameterValue` _returnvalue_5 "Amount" `_새_트랙_0_2`))
        (:`Finished`
          (`self.K2_DestroyActor`))))))

(fn `UserConstructionScript`)