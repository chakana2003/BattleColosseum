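; BP_FieldItem is an item actor placed or spawned in the field, holding an item class ID and stack count.
; LoadItem, or BeginPlay when the ID is already non-zero, looks up the ID's row in the new item data table.
; It then async loads and applies the row's static mesh and resizes the sphere component to that mesh's bounds radius.
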(event `LoadItem`
  (params (ItemClassID :type Integer) (StackCount :type Integer))
  (bind _staticmeshcomponent (`self.StaticMeshComponent`))
  (set `self.ItemClassID` ItemClassID)
  (set `self.StackCount` StackCount)
  (bind _returnvalue (`|GetDataTableRow` "/Game/Wonseok/NewInventory/NewItemDataTable.NewItemDataTable" (`KismetStringLibrary.Conv_StringToName` (`KismetStringLibrary.Conv_IntToString` (`self.ItemClassID`))) :!label _label)
    (:`then`
      (bind _object (`|LoadAsset` (`.StaticMesh_12_690FECB144EC4A97085B61819D64D421` (break `/Game/Wonseok/NewInventory/ItemClass` _returnvalue)))
        (:`Completed`
          (bind _asstatic_mesh (cast `StaticMesh` _object))
          (`StaticMeshComponent.SetStaticMesh` _staticmeshcomponent _asstatic_mesh)
          (`SphereComponent.SetSphereRadius` (`self.Sphere`) (`.SphereRadius` (`KismetSystemLibrary.GetComponentBounds` _staticmeshcomponent)) true))))))

(event `self.ReceiveBeginPlay`
  (if (!= (`self.ItemClassID`) 0)
    (goto _label)))

(fn `UserConstructionScript`)